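; Blueprint Interface for close-combat targets, defining the calls used to query and notify a combatant without knowing its class.
; Queries expose attack and fatality state, weapon vector and impulse, damage animation type, skills, block and avoid multipliers, combat state and health.
; Calls without outputs cover death with an XP value, blocking, retargeting, fatalities, victim animations and stealth kills.
; It holds only signatures, with behavior left to implementers.
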(fn TargetIsAttack
  (return false false))

(fn TargetWeaponVec
  (return "0, 0, 0" 0.0))

(fn TargetDamageTypeAnim
  (return "NewEnumerator0"))

(fn TargetIsDead
  (params (XPvalue :type Float%20%28single-precision%29)))

(fn TargetFatality
  (params (Target :type Actor%20Object%20Reference) (Stealth :type Boolean)))

(fn TargetBlock)

(fn TargetGetSkill
  (params (SkillName :type String))
  (return "" false false))

(fn TargetAttackParameters
  (return 0.0 0.0 0))

(fn TargetCombatState
  (return false false false))

(fn TargetStealthKill
  (params (DamageCauser :type Actor%20Object%20Reference)))

(fn TargetHealth
  (return 0.0 0.0))

(fn TargetSetNewTarget
  (params (Target :type Actor%20Object%20Reference)))

(fn TargetFatalityVictimAnimation
  (params (Stealth :type Boolean) (Index :type Integer) (FatalityType :type String)))
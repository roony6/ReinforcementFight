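; BPC_GreyStone_EnemyS is a GreyStone NPC character that locks onto an overlapping BPC_GreyStone_EnemyS1 as its opponent.
; A box overlap stores the opponent, and a looping timer, used instead of Tick, turns the actor to face it by yaw only.
; A second timer regenerates stamina while not attacking or dodging, refreshing it through UpdateStamina.
; A helper derives TurnValue from yaw change but is not called here.
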(event OnComponentBeginOverlap(Box)
  (params (OverlappedComponent :type Primitive%20Component%20Object%20Reference) (OtherActor :type Actor%20Object%20Reference) (OtherComp :type Primitive%20Component%20Object%20Reference) (OtherBodyIndex :type Integer) (bFromSweep :type Boolean) (SweepResult :type Hit%20Result%20Structure%20%28by%20ref%29))
  (bind _asbpc_grey_stone_enemy_s1 (Utilities|Casting|CastToBPC_GreyStone_EnemyS1 OtherActor))
  (Variables|Default|Setopponent _asbpc_grey_stone_enemy_s1))

(event Custom|StaminaReg
  (if (Math|Boolean|ANDBoolean (not (Variables|Default|GetIsAttacking)) (not (Variables|Default|GetisDodging)) (not (== (Variables|Default|GetCurrentStamina) (Variables|Default|GetMaxStamina))))
    (Variables|Default|SetCurrentStamina (+ (Variables|Default|GetCurrentStamina) (Variables|Default|GetStaminaReGen)))
    (CallFunction|UpdateStamina)))

(event Custom|CustomEventick
  (bind _opponent (Variables|Default|Getopponent))
  (Utilities|IsValid _opponent
    (:Is%20Valid
      (Utilities|LookatPlayer _opponent))))

(event EventBeginPlay
  (CallFunction|UpdateHealth)
  (CallFunction|UpdateStamina)
  (Utilities|Time|SetTimerbyEvent (delegate Custom|CustomEventick) (* (Variables|Default|GetCurrentTickTime) (Variables|Default|GetCurrentTickTimeMultiply)) true)
  (Utilities|Time|SetTimerbyEvent (delegate Custom|StaminaReg) 0.2 true))

(fn ConstructionScript
  (|CallParentFunction))
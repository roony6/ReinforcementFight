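; Randomized GreyStone enemy character that starts with its sword equipped and tracks the player pawn.
; BeginPlay caches its animation Blueprint and game instance, then starts looping timers for distance tracking and stamina regeneration.
; Distance to the player, plus distance walked when not dodging, is written to the game instance; stamina regenerates outside attacks and dodges.
; Helper functions provide yaw-only look-at rotation and a turn value from yaw change.
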(event Custom|StaminaReg
  ;[0.03088 0 1] Stamina Reg
  (if (Math|Boolean|ANDBoolean (not (Variables|Default|GetIsAttacking)) (not (Variables|Default|GetisDodging)) (not (== (Variables|Default|GetCurrentStamina) (Variables|Default|GetMaxStamina))))
    (Variables|Default|SetCurrentStamina (+ (Variables|Default|GetCurrentStamina) (Variables|Default|GetStaminaReGen)))
    (CallFunction|UpdateStamina)))

(event Custom|UpdateDistance
  (bind _game_instance (Variables|Default|GetGame%20instance))
  ;[0.5 0.476 0] Update Distance
  (Variables|/Game/Character/B_GameInstance.B_GameInstance_C|SetOldDistanceToPlayer _game_instance (Variables|/Game/Character/B_GameInstance.B_GameInstance_C|GetDistanceToPlayer _game_instance))
  (bind _distance (CallFunction|DistancetoTarget (Variables|Default|GetPlayerRefrence)))
  (Variables|/Game/Character/B_GameInstance.B_GameInstance_C|SetDistanceToPlayer (Variables|Default|GetGame%20instance) _distance)
  (if (not (Variables|Default|GetisDodging))
    (Variables|/Game/Character/B_GameInstance.B_GameInstance_C|SetDistanceWalked (Variables|Default|GetGame%20instance) (Math|Float|Truncate (* (Math|Vector|VectorLength (Transformation|GetVelocity)) 0.2)))))

(event EventTick
  (params (DeltaSeconds :type Float%20%28single-precision%29))
  (|CallParentFunction DeltaSeconds))

(event EventBeginPlay
  (Variables|Default|SetSwordEquiped true)
  (Variables|Default|SetPlayerRefrence (Pawn|GetControlledPawn (Game|GetPlayerController 0)))
  (bind _asabp_grey_stone (Utilities|Casting|CastToABP_GreyStone (Components|SkeletalMesh|GetAnimInstance (Variables|Character|GetMesh))))
  (Variables|Default|SetAnimationBP _asabp_grey_stone)
  (CallFunction|UpdateHealth)
  (CallFunction|UpdateStamina)
  (bind _asb_game_instance (Utilities|Casting|CastToB_GameInstance (Game|GetGameInstance)))
  (Variables|Default|SetGame%20instance _asb_game_instance)
  ;[0.5 0.476 0] Update Distance
  (Utilities|Time|SetTimerbyEvent (delegate Custom|UpdateDistance) 0.2 true)
  ;[0.03088 0 1] Stamina Reg
  (Utilities|Time|SetTimerbyEvent (delegate Custom|StaminaReg) 0.3 true))

(fn ConstructionScript
  (|CallParentFunction))
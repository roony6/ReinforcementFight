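; Prototype enemy character that turns to face the player's pawn.
; On BeginPlay it caches the pawn, updates health and starts a looping timer that snaps yaw toward the player, in place of Tick.
; Helpers measure and print player distance or wrap AI Move To with a MovedTo flag, passing the player controller as target actor.
; Directional roll montages are unwired, and MoveToLocation in the event graph is an empty stub.
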(event Custom|CustomEventTick
  (Transformation|SetActorRotation (Math|Rotator|MakeRotator 0.0 0.0 (.yaw (Math|Rotator|FindLookatRotation (Transformation|GetActorLocation) (Transformation|GetActorLocation (Variables|Default|GetPlayerRefrence))))) true))

(event Custom|DistancePlayer
  (bind _output_get (Variables|Default|SetDistanceToPlayer (Math|Float|Truncate (Transformation|GetDistanceTo (Variables|Default|GetPlayerRefrence)))))
  (Development|PrintString (Utilities|String|Append "Distance To Player" "  : " (Utilities|String|ToString(Integer) _output_get))))

(event EventBeginPlay
  (Variables|Default|SetPlayerRefrence (Pawn|GetControlledPawn (Game|GetPlayerController 0)))
  (CallFunction|UpdateHealth)
  (Utilities|Time|SetTimerbyEvent (delegate Custom|CustomEventTick) (* (Variables|Default|GetCustomTickTime) (Variables|Default|GetCustomTickTimeMultiply)) true))

(fn ConstructionScript
  (|CallParentFunction))

(fn DistancetoTarget
  (params (Target :type Actor%20Object%20Reference))
  (bind _output_get (Variables|Default|SetDistanceToPlayer (Math|Float|Truncate (Transformation|GetDistanceTo Target))))
  (Development|PrintString (Utilities|String|Append "Distance To Player" "  : " (Utilities|String|ToString(Integer) _output_get)) true true "(R=0.000000,G=0.660000,B=1.000000,A=1.000000)" 0.0)
  (return _output_get))

(event EventMovetoLocation
  (params (Location :type Vector :default "0, 0, 0"))
  (Variables|Default|SetMovedTo false)
  (AI|AIMoveTo self Location (Game|GetPlayerController 0) 5e+01 false
    (:OnSuccess
      (Variables|Default|SetMovedTo true)
      (return))))